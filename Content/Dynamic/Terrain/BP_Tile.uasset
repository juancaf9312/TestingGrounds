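; BP_Tile is a terrain tile for an endlessly extending Testing Grounds level, scattering props such as containers, rocks and trees through PlaceActors on BeginPlay.
; Player overlap with CollisionBox opens the Barrier and turns it green.
; Leaving it closes the red barrier, asks the game mode to spawn another tile and shows the Wall.
; Overlapping DestroyBox destroys the tile, while GetAttachLocation exposes the Arrow transform as an attach point.
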(event OnComponentBeginOverlap(CollisionBox)
  (params (OverlappedComponent :type Primitive%20Component%20Object%20Reference) (OtherActor :type Actor%20Object%20Reference) (OtherComp :type Primitive%20Component%20Object%20Reference) (OtherBodyIndex :type Integer) (bFromSweep :type Boolean) (SweepResult :type Hit%20Result%20Structure%20%28by%20ref%29))
  (Utilities|IsPlayer OtherActor)
  (Collision|SetCollisionEnabled (Variables|Default|GetBarrier) "NoCollision")
  (Rendering|Material|SetMaterial (Variables|Default|GetBarrier) 0 "/Game/Dynamic/Terrain/MI_Barrier_Green.MI_Barrier_Green"))

(event OnComponentEndOverlap(CollisionBox)
  (params (OverlappedComponent :type Primitive%20Component%20Object%20Reference) (OtherActor :type Actor%20Object%20Reference) (OtherComp :type Primitive%20Component%20Object%20Reference) (OtherBodyIndex :type Integer))
  (Utilities|IsPlayer OtherActor)
  (Collision|SetCollisionEnabled (Variables|Default|GetBarrier) "QueryAndPhysics")
  (Rendering|Material|SetMaterial (Variables|Default|GetBarrier) 0 "/Game/Dynamic/Terrain/MI_Barrier_Red.MI_Barrier_Red")
  (bind _asbp_testing_grounds_game_mode (Utilities|Casting|CastToBP_TestingGroundsGameMode (Game|GetGameMode)))
  (Default|SpawnTile _asbp_testing_grounds_game_mode)
  (Rendering|SetVisibility (Variables|Default|GetWall) true false))

(event OnComponentBeginOverlap(DestroyBox)
  (params (OverlappedComponent :type Primitive%20Component%20Object%20Reference) (OtherActor :type Actor%20Object%20Reference) (OtherComp :type Primitive%20Component%20Object%20Reference) (OtherBodyIndex :type Integer) (bFromSweep :type Boolean) (SweepResult :type Hit%20Result%20Structure%20%28by%20ref%29))
  (Utilities|IsPlayer OtherActor)
  (Actor|DestroyActor))

(event EventBeginPlay
  (Collision|SetCollisionEnabled (Variables|Default|GetBarrier) "QueryAndPhysics")
  (Class|Tile|PlaceActors "/Game/Dynamic/Terrain/Props/BP_Container.BP_Container_C" 1 2 4e+02 1.0 1.0)
  (Class|Tile|PlaceActors "/Game/Dynamic/Terrain/Props/BP_Box.BP_Box_C" 2 3 1e+02 1.0 1.0)
  (Class|Tile|PlaceActors "/Game/Dynamic/Terrain/Props/BP_Canister.BP_Canister_C" 1 4 5e+01 1.0 1.0)
  (Class|Tile|PlaceActors "/Game/Dynamic/Terrain/Props/BP_Rock01.BP_Rock01_C" 1 3 1.5e+02 0.5 5.0)
  (Class|Tile|PlaceActors "/Game/Dynamic/Terrain/Props/BP_Rock05.BP_Rock05_C" 1 3 2.5e+02 0.5 5.0)
  (Class|Tile|PlaceActors "/Game/Dynamic/Terrain/Props/BP_Rock17.BP_Rock17_C" 1 3 2.5e+02 0.5 5.0)
  (Class|Tile|PlaceActors "/Game/Dynamic/Terrain/Props/BP_SackWall.BP_SackWall_C" 1 2 2.5e+02 1.0 1.0)
  (Class|Tile|PlaceActors "/Game/Dynamic/Terrain/Props/BP_Tree.BP_Tree_C" 1 8 2e+02 0.8 1.2)
  (Class|Tile|PlaceActors "/Game/Dynamic/Terrain/Props/BP_ScaffFolding.BP_ScaffFolding_C" 1 2 5e+02 1.0 1.0))

(event Collision|EventActorBeginOverlap
  (params (OtherActor :type Actor%20Object%20Reference)))

(event EventTick
  (params (DeltaSeconds :type Float%20%28single-precision%29)))

(fn ConstructionScript)

(fn GetAttachLocation
  (return (Transformation|GetWorldTransform (Variables|Default|GetArrow))))
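; BP_NPC_AI is an AI controller for guard NPCs that reacts to perceived targets.
; On BeginPlay it loads the patrol blackboard and runs the GuardBehaviour behavior tree.
; AI perception updates ignore actors tagged "AI"; sensing any other stores it as the enemy key and turns on the pawn's Aiming and Shooting flags.
; Losing the stimulus clears the key and both flags.
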(event OnTargetPerceptionUpdated(AIPerception)
  (params (Actor :type Actor%20Object%20Reference) (Stimulus :type AI%20Stimulus%20Structure))
  (bind _returnvalue (Pawn|GetControlledPawn))
  (bind _ascharacter (Utilities|Casting|CastToCharacter _returnvalue))
  (if (not (Actor|ActorHasTag Actor "AI"))
    (if (.bSuccessfullySensed (Utilities|Struct|BreakAIStimulus Stimulus))
      (AI|Components|Blackboard|SetValueasObject (Variables|Default|GetBlackboardComp) (Variables|Default|GetEnemyKey) Actor)
      (Variables|/Game/Dynamic/Character/Behaviour/Character.Character_C|SetAiming _ascharacter true)
      (Variables|/Game/Dynamic/Character/Behaviour/Character.Character_C|SetShooting _ascharacter true)
      (else
        (AI|Components|Blackboard|ClearValue (Variables|Default|GetBlackboardComp) (Variables|Default|GetEnemyKey))
        (Variables|/Game/Dynamic/Character/Behaviour/Character.Character_C|SetAiming _ascharacter false)
        (Variables|/Game/Dynamic/Character/Behaviour/Character.Character_C|SetShooting _ascharacter false)))))

(event EventBeginPlay
  (bind _blackboardcomponent (Class|AIController|UseBlackboard "/Game/Dynamic/Character/AI/BB_PatrolData.BB_PatrolData"))
  (Variables|Default|SetBlackboardComp _blackboardcomponent)
  (AI|RunBehaviorTree "/Game/Dynamic/Character/AI/GuardBehaviour.GuardBehaviour"))

(event EventTick
  (params (DeltaSeconds :type Float%20%28single-precision%29)))

(fn ConstructionScript)
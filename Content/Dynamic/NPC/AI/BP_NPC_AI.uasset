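; AI controller for NPCs that runs the GuardBehaviour behavior tree on the BB_PatrolData blackboard, started on BeginPlay.
; AI perception updates store any sensed actor without the "AI" tag in the enemy blackboard key, and clear the key when sensing is lost.
; The same updates switch the controlled Ue4ASP_Character's Aiming flag on and off.
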(event OnTargetPerceptionUpdated(AIPerception)
  (params (Actor :type Actor%20Object%20Reference) (Stimulus :type AI%20Stimulus%20Structure))
  (bind _returnvalue (Pawn|GetControlledPawn))
  (bind _asue_4asp_character (Utilities|Casting|CastToUe4ASP_Character _returnvalue))
  (if (not (Actor|ActorHasTag Actor "AI"))
    (if (.bSuccessfullySensed (Utilities|Struct|BreakAIStimulus Stimulus))
      (AI|Components|Blackboard|SetValueasObject (Variables|Default|GetBlackboardComp) (Variables|Default|GetEnemyKey) Actor)
      (Variables|/Game/Dynamic/NPC/Behaviour/Ue4ASP_Character.Ue4ASP_Character_C|SetAiming _asue_4asp_character true)
      (else
        (AI|Components|Blackboard|ClearValue (Variables|Default|GetBlackboardComp) (Variables|Default|GetEnemyKey))
        (Variables|/Game/Dynamic/NPC/Behaviour/Ue4ASP_Character.Ue4ASP_Character_C|SetAiming _asue_4asp_character false)))))

(event EventBeginPlay
  (bind _blackboardcomponent (Class|AIController|UseBlackboard "/Game/Dynamic/NPC/AI/BB_PatrolData.BB_PatrolData"))
  (Variables|Default|SetBlackboardComp _blackboardcomponent)
  (AI|RunBehaviorTree "/Game/Dynamic/NPC/AI/GuardBehaviour.GuardBehaviour"))

(event EventTick
  (params (DeltaSeconds :type Float%20%28single-precision%29)))

(fn ConstructionScript)